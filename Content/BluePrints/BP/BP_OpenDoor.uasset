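; BP_OpenDoor is a door that opens when the mass of actors inside its linked Trigger reaches a threshold.
; Each overlap begin recomputes Masse by summing the static mesh masses of the trigger's overlapping actors, while any overlap end resets it to zero.
; Tick compares Masse to the threshold every frame, sets IsDoorOpen and snaps the actor between two fixed rotations without interpolation.
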(event OnActorBeginOverlap(trigger)
  (params (OverlappedActor :type Actor%20Object%20Reference) (OtherActor :type Actor%20Object%20Reference))
  ;[1 1 1] Si un acteur se trouve dans le trigger, le trigger prend la valeur de sa masse
  (Variables|Default|SetMasse 0.0)
  (CallFunction|SetMasse OverlappedActor))

(event OnActorEndOverlap(trigger)
  (params (OverlappedActor :type Actor%20Object%20Reference) (OtherActor :type Actor%20Object%20Reference))
  ;[1 1 1] Quand l'actreur quitte le trigger, remet la masse à 0
  (Variables|Default|SetMasse 0.0))

(event EventTick
  (params (DeltaSeconds :type Float%20%28single-precision%29))
  ;[1 1 1] Si la casse est supperieur à 120, la porte s'ouvre
  (if (>= (Variables|Default|GetMasse) 1.2e+02)
    (Variables|Default|SetIsDoorOpen true)
    (Transformation|SetActorRotation "0,0.000000, 0")
    (else
      (Variables|Default|SetIsDoorOpen false)
      (Transformation|SetActorRotation "0,-90.000000, 0"))))

(fn ConstructionScript)

(fn SetMasse
  (params (Target :type Actor%20Object%20Reference))
  ;[1 1 1] Prend la valeur de la masse des acteur dans le trigger volume
  (bind _output_get (Variables|Default|SetActors (Collision|GetOverlappingActors Target 0 :!class /Script/Engine.Actor)))
  (for _array_element _output_get
    (Variables|Default|SetMasse (+ (Variables|Default|GetMasse) (Physics|GetMass (Actor|GetComponentbyClass _array_element "/Script/Engine.StaticMeshComponent"))))))